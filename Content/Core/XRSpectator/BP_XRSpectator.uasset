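; BP_XRSpectator is an XR spectator actor that shows a render target on the spectator screen and smoothly follows a given scene component.
; BeginPlay switches the spectator screen to texture mode using RT_XRSpectator.
; StartCameraFollow waits a tick, then starts a looping timer whose interval is that moment's frame delta, used instead of Tick.
; Each timer call interpolates the actor's transform toward the component's world transform to smooth the motion.
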(event `self.ReceiveBeginPlay`
  (`HeadMountedDisplayFunctionLibrary.SetSpectatorScreenMode` "Texture")
  (`HeadMountedDisplayFunctionLibrary.SetSpectatorScreenTexture` "/Game/Core/XRSpectator/RT_XRSpectator.RT_XRSpectator"))

(event `StartCameraFollow`
  (params (SceneComponent :type "SceneComponent Object Reference"))
  (`KismetSystemLibrary.DelayUntilNextTick`)
  (`KismetSystemLibrary.K2_SetTimerDelegate` (delegate `CameraFollow`) (`GameplayStatics.GetWorldDeltaSeconds`) true))

(event `CameraFollow`
  (`self.SetSpectatorTransform` (stale `StartCameraFollow` SceneComponent)))

(fn `SetSpectatorTransform`
  (params (SceneComponent :type "SceneComponent Object Reference"))
  (`self.K2_SetActorTransform` (`KismetMathLibrary.TInterpTo` (`self.GetTransform`) (`SceneComponent.K2_GetComponentToWorld` SceneComponent) (`GameplayStatics.GetWorldDeltaSeconds`) 15.0)))

(fn `UserConstructionScript`)
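; BP_3DLabel is a world-space label actor that keeps turning to face the XR player's camera.
; On BeginPlay and every Tick, it points its Widget fully at the BP_XR_Character camera using a look-at rotation.
; It also turns the actor on yaw only toward the camera with a fixed angular offset, preserving its pitch and roll.
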(event `self.ReceiveBeginPlay`
  (bind (_returnvalue_roll _returnvalue_pitch) (`KismetMathLibrary.BreakRotator` (`self.K2_GetActorRotation`)))
  (bind _asbp_xr_character (cast `/Game/Character/BP_XR_Character` (`GameplayStatics.GetPlayerPawn` 0)))
  (bind _returnvalue (`KismetMathLibrary.FindLookAtRotation` (`self.K2_GetActorLocation`) (`SceneComponent.K2_GetComponentLocation` (`/Game/Character/BP_XR_Character.Camera` _asbp_xr_character))))
  (`SceneComponent.K2_SetWorldRotation` (`self.Widget`) _returnvalue false false)
  (`self.K2_SetActorRotation` (`KismetMathLibrary.MakeRotator` _returnvalue_roll _returnvalue_pitch (+ (.yaw _returnvalue) 25.0))))

(event `self.ReceiveTick`
  (params (DeltaSeconds :type "Float (single-precision)"))
  (bind (_returnvalue_roll _returnvalue_pitch) (`KismetMathLibrary.BreakRotator` (`self.K2_GetActorRotation`)))
  (bind _asbp_xr_character (cast `/Game/Character/BP_XR_Character` (`GameplayStatics.GetPlayerPawn` 0)))
  (bind _returnvalue (`KismetMathLibrary.FindLookAtRotation` (`self.K2_GetActorLocation`) (`SceneComponent.K2_GetComponentLocation` (`/Game/Character/BP_XR_Character.Camera` _asbp_xr_character))))
  (`SceneComponent.K2_SetWorldRotation` (`self.Widget`) _returnvalue false false)
  (`self.K2_SetActorRotation` (`KismetMathLibrary.MakeRotator` _returnvalue_roll _returnvalue_pitch (+ (.yaw _returnvalue) 25.0))))

(fn `UserConstructionScript`)
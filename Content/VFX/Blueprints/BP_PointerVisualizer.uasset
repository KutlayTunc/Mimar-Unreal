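; BP_PointerVisualizer drives a Niagara curved beam that visualizes a pointer, with an end point that trails the aim direction.
; Starting updates snaps the end along the beam's forward vector, using the obstructed length if set, else the default, and starts a looping timer at frame delta.
; Each tick interpolates the world-space end toward that target, converts it to local space for Niagara, and broadcasts the pointer location update until stopped.
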(event `StartUpdatingBeamEnd`
  (bind _returnvalue (+ (* (`SceneComponent.GetForwardVector` (`self.CurveBeam`)) (select `bool` (> (`self.ObstructedBeamLenght`) 1.0) :`false` (`self.BeamLength`) :`true` (`self.ObstructedBeamLenght`))) (`SceneComponent.K2_GetComponentLocation` (`self.CurveBeam`))))
  (`NiagaraComponent.SetNiagaraVariableVec3` (`self.CurveBeam`) (`self.NiagaraBeamEnd`) (`KismetMathLibrary.InverseTransformLocation` (`SceneComponent.K2_GetComponentToWorld` (`self.CurveBeam`)) _returnvalue))
  (set `self.CurrentBeamEndWorldLocation` _returnvalue)
  (bind _returnvalue_2 (`KismetSystemLibrary.K2_SetTimerDelegate` (delegate `StartTimerUpdateBeamEnd`) (`GameplayStatics.GetWorldDeltaSeconds`) true))
  (set `self.BeamEndUpdaterTimer` _returnvalue_2))

(event `StartTimerUpdateBeamEnd`
  (bind _curvebeam (`self.CurveBeam`))
  (bind _returnvalue (`KismetMathLibrary.VInterpTo` (`self.CurrentBeamEndWorldLocation`) (+ (* (`SceneComponent.GetForwardVector` _curvebeam) (select `bool` (> (`self.ObstructedBeamLenght`) 1.0) :`false` (`self.BeamLength`) :`true` (`self.ObstructedBeamLenght`))) (`SceneComponent.K2_GetComponentLocation` _curvebeam)) (`GameplayStatics.GetWorldDeltaSeconds`) 4.0))
  (`NiagaraComponent.SetNiagaraVariableVec3` (`self.CurveBeam`) (`self.NiagaraBeamEnd`) (`KismetMathLibrary.InverseTransformLocation` (`SceneComponent.K2_GetComponentToWorld` (`self.CurveBeam`)) _returnvalue))
  (set `self.CurrentBeamEndWorldLocation` _returnvalue)
  (`self.PointerLocationUpdated`))

(event `StopUpdatingBeamEnd`
  (`KismetSystemLibrary.K2_ClearAndInvalidateTimerHandle` (`self.BeamEndUpdaterTimer`)))

(fn `UserConstructionScript`)
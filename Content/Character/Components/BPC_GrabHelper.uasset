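; Grab helper component that lets two hands move, scale and rotate a target static mesh together.
; BeginPlay snapshots the hands' midpoint, spacing and orientation basis along with the mesh's transform, rather than capturing them when a grab starts.
; While both grab flags are set, Tick moves the mesh with the midpoint, scales it by the clamped spacing ratio and rotates it using a basis built from hand direction and averaged up vectors.
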(event `self.ReceiveTick`
  (params (DeltaSeconds :type "Float (single-precision)"))
  (`self.UpdateGrabLogic`))

(event `self.ReceiveBeginPlay`
  (set `self.TargetMesh` (`StaticMeshActor.StaticMeshComponent` (`self.TargetMeshActor`)))
  (bind _output_get (set `self.RightGrabLocation` (`SceneComponent.K2_GetComponentLocation` (`self.R_Hand`))))
  (bind _output_get_2 (set `self.LeftGrabLocation` (`SceneComponent.K2_GetComponentLocation` (`self.L_Hand`))))
  (bind _output_get_3 (set `self.InitialDirection` (- _output_get _output_get_2)))
  (set `self.InitialGrabDistance` (`KismetMathLibrary.VSize` _output_get_3))
  (bind _output_get_4 (set `self.InitialCentroid` (* (+ (`self.RightGrabLocation`) (`self.LeftGrabLocation`)) 0.5)))
  (set `self.InitialMeshOffset` (- (`SceneComponent.K2_GetComponentLocation` (`self.TargetMesh`)) _output_get_4))
  (set `self.InitialHandsForward` (`KismetMathLibrary.Normal` (`self.InitialDirection`)))
  (bind _output_get_5 (set `self.InitialHandsUp` (`KismetMathLibrary.Normal` (* (+ (`KismetMathLibrary.GetUpVector` (`SceneComponent.K2_GetComponentRotation` (`self.L_Hand`))) (`KismetMathLibrary.GetUpVector` (`SceneComponent.K2_GetComponentRotation` (`self.R_Hand`)))) 0.5))))
  (bind _output_get_6 (set `self.InitialHandsUp` (`KismetMathLibrary.Normal` (`KismetMathLibrary.Vector_ProjectOnToNormal` _output_get_5 (`self.InitialHandsForward`)))))
  (bind _output_get_7 (set `self.InitialHandsRight` (`KismetMathLibrary.Cross_VectorVector` (`self.InitialHandsForward`) _output_get_6)))
  (set `self.InitialHandsUp` (`KismetMathLibrary.Cross_VectorVector` _output_get_7 (`self.InitialHandsForward`)))
  (set `self.InitialLeftHandRotation` (`SceneComponent.K2_GetComponentRotation` (`self.L_Hand`)))
  (set `self.InitialRightHandRotation` (`SceneComponent.K2_GetComponentRotation` (`self.R_Hand`)))
  (set `self.InitialMeshRotation` (`SceneComponent.K2_GetComponentRotation` (`self.TargetMesh`)))
  (set `self.InitialScale` (`SceneComponent.K2_GetComponentScale` (`self.TargetMesh`)))
  (set `self.InitialHandsRotation` (`KismetMathLibrary.MakeRotFromXY` (`self.InitialHandsForward`) (`self.InitialHandsRight`)))
  (set `self.LastMeshRotation` (`SceneComponent.K2_GetComponentRotation` (`self.TargetMesh`))))

(fn `SetHands`
  (params (R_Hand :type "SceneComponent Object Reference") (L_Hand :type "SceneComponent Object Reference"))
  (set `self.R_Hand` R_Hand)
  (set `self.L_Hand` L_Hand))

(fn `UpdateGrabLogic`
  (locals (CurrentDistance :type "Float (double-precision)" :default 0.0) (ScaleFactor :type "Float (double-precision)") (NewScale :type "Vector Structure") (DeltaRotation :type "Rotator Structure" :default (struct)) (CurrentCentroid :type "Vector Structure") (CurrentHandsRotation :type "Rotator Structure" :default (struct)) (LeftTwist :type "Rotator Structure" :default (struct)) (RightTwist :type "Rotator Structure" :default (struct)) (RightHandPos :type "Vector Structure" :default (0.0 0.0 0.0)) (LeftHandPos :type "Vector Structure" :default (0.0 0.0 0.0)) (CurrentHandsForward :type "Vector Structure" :default (0.0 0.0 0.0)) (LeftUpVector :type "Vector Structure" :default (0.0 0.0 0.0)) (RightUpVector :type "Vector Structure" :default (0.0 0.0 0.0)) (CurrentHandsUp :type "Vector Structure" :default (0.0 0.0 0.0)) (CurrentHandsRight :type "Vector Structure" :default (0.0 0.0 0.0)) (AverageTwist :type "Rotator Structure" :default (struct)) (LeftHandRot :type "Rotator Structure" :default (struct)) (RightHandRot :type "Rotator Structure" :default (struct)) (NewLocation :type "Vector Structure") (TwistRotation :type "Rotator Structure" :default (struct)))
  (bind _initialscale_x (`KismetMathLibrary.BreakVector` (`self.InitialScale`)))
  (if (and (`self.isGrabbedLeft`) (`self.isGrabbedRight`))
    ;[0.15 0.09008 0.03888 0.5] Location
    (set `local.LeftHandPos` (`SceneComponent.K2_GetComponentLocation` (`self.L_Hand`)))
    (set `local.RightHandPos` (`SceneComponent.K2_GetComponentLocation` (`self.R_Hand`)))
    (set `local.LeftHandRot` (`SceneComponent.K2_GetComponentRotation` (`self.L_Hand`)))
    (set `local.RightHandRot` (`SceneComponent.K2_GetComponentRotation` (`self.R_Hand`)))
    (bind _output_get (set `local.CurrentCentroid` (* (+ (`local.LeftHandPos`) (`local.RightHandPos`)) 0.5)))
    (bind _output_get_2 (set `local.NewLocation` (+ _output_get (`self.InitialMeshOffset`))))
    (`SceneComponent.K2_SetWorldLocation` (`self.TargetMesh`) _output_get_2 false false)
    ;[0.01659 0.109 0.15 0.5] Scale
    (bind _output_get_3 (set `local.CurrentDistance` (`KismetMathLibrary.VSize` (- (`local.RightHandPos`) (`local.LeftHandPos`)))))
    (bind _output_get_4 (set `local.ScaleFactor` (/ _output_get_3 (`self.InitialGrabDistance`))))
    (`SceneComponent.SetWorldScale3D` (`self.TargetMesh`) (`KismetMathLibrary.ClampVectorSize` (* _output_get_4 (`self.InitialScale`)) 0.1 (* _initialscale_x 5.0)))
    ;[0.09237 0.05267 0.15 0.5] Rotation
    (set `local.CurrentHandsForward` (`KismetMathLibrary.Normal` (- (`local.RightHandPos`) (`local.LeftHandPos`))))
    (bind _output_get_5 (set `local.CurrentHandsUp` (`KismetMathLibrary.Normal` (* (+ (`KismetMathLibrary.GetUpVector` (`local.LeftHandRot`)) (`KismetMathLibrary.GetUpVector` (`local.RightHandRot`))) 0.5))))
    (bind _output_get_6 (set `local.CurrentHandsUp` (`KismetMathLibrary.Normal` (`KismetMathLibrary.Vector_ProjectOnToNormal` _output_get_5 (`local.CurrentHandsForward`)))))
    (bind _output_get_7 (set `local.CurrentHandsRight` (`KismetMathLibrary.Cross_VectorVector` (`local.CurrentHandsForward`) _output_get_6)))
    (set `local.CurrentHandsUp` (`KismetMathLibrary.Cross_VectorVector` _output_get_7 (`local.CurrentHandsForward`)))
    (set `local.CurrentHandsRotation` (`KismetMathLibrary.MakeRotFromXY` (`local.CurrentHandsForward`) (`local.CurrentHandsRight`)))
    (`SceneComponent.K2_SetWorldRotation` (`self.TargetMesh`) (`KismetMathLibrary.ComposeRotators` (`KismetMathLibrary.NormalizedDeltaRotator` (`self.InitialMeshRotation`) (`self.InitialHandsRotation`)) (`local.CurrentHandsRotation`)) false false)
    (set `self.LeftGrabLocation` (`local.LeftHandPos`))
    (set `self.RightGrabLocation` (`local.RightHandPos`))))
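; BP_PCTEST_Character is a character Blueprint, named as a PC test, that drives hand grabbing from the keyboard.
; The construction script passes its right and left hand components to the BPCGrabHelper component.
; Q and E each use a FlipFlop to toggle that component's left and right grabbed flags, so each press switches between grabbed and released.
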(event Collision|EventActorBeginOverlap
  (params (OtherActor :type Actor%20Object%20Reference)))

(event EventTick
  (params (DeltaSeconds :type Float%20%28single-precision%29)))

(event EventBeginPlay)

(event Input|KeyboardEvents|E
  (params (Key :type Key%20Structure :default "None"))
  (bind _bpc_grabhelper (Variables|Default|GetBPC_GrabHelper))
  (:Pressed
    (Utilities|FlowControl|FlipFlop
      (:A
        (Variables|/Game/Character/Components/BPC_GrabHelper.BPC_GrabHelper_C|SetisGrabbedRight _bpc_grabhelper true))
      (:B
        (Variables|/Game/Character/Components/BPC_GrabHelper.BPC_GrabHelper_C|SetisGrabbedRight _bpc_grabhelper false)))))

(event Input|KeyboardEvents|Q
  (params (Key :type Key%20Structure :default "None"))
  (bind _bpc_grabhelper (Variables|Default|GetBPC_GrabHelper))
  (:Pressed
    (Utilities|FlowControl|FlipFlop
      (:A
        (Variables|/Game/Character/Components/BPC_GrabHelper.BPC_GrabHelper_C|SetisGrabbedLeft _bpc_grabhelper true))
      (:B
        (Variables|/Game/Character/Components/BPC_GrabHelper.BPC_GrabHelper_C|SetisGrabbedLeft _bpc_grabhelper false)))))

(fn ConstructionScript
  (Default|SetHands (Variables|Default|GetBPC_GrabHelper) (Variables|Default|GetR_Hand) (Variables|Default|GetL_Hand)))
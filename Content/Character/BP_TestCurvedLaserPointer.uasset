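; Test actor for a curved laser pointer, driving the end point of a Niagara beam so it lags behind the component's aim.
; BeginPlay places the beam end 100 units along the Niagara component's forward vector.
; Each Tick eases the stored world-space end toward that forward point with VInterpTo, then passes it to the BeamEnd variable converted into the component's local space.
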(event `self.ReceiveBeginPlay`
  (bind _niagara (`self.Niagara`))
  (bind _returnvalue (+ (* (`SceneComponent.GetForwardVector` _niagara) 100.0) (`SceneComponent.K2_GetComponentLocation` _niagara)))
  (`NiagaraComponent.SetNiagaraVariableVec3` (`self.Niagara`) "BeamEnd" (`KismetMathLibrary.InverseTransformLocation` (`SceneComponent.K2_GetComponentToWorld` (`self.Niagara`)) _returnvalue))
  (set `self.CurrentBeamEndLocation` _returnvalue))

(event `self.ReceiveTick`
  (params (DeltaSeconds :type "Float (single-precision)"))
  (bind _niagara (`self.Niagara`))
  (bind _returnvalue (`KismetMathLibrary.VInterpTo` (`self.CurrentBeamEndLocation`) (+ (* (`SceneComponent.GetForwardVector` _niagara) 100.0) (`SceneComponent.K2_GetComponentLocation` _niagara)) DeltaSeconds 2.0))
  (`NiagaraComponent.SetNiagaraVariableVec3` (`self.Niagara`) "BeamEnd" (`KismetMathLibrary.InverseTransformLocation` (`SceneComponent.K2_GetComponentToWorld` (`self.Niagara`)) _returnvalue))
  (set `self.CurrentBeamEndLocation` _returnvalue))

(fn `UserConstructionScript`)
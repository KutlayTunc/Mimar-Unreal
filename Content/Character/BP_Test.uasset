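; Test Blueprint for two-handed manipulation, moving, rotating and scaling Object from the Left and Right components.
; BeginPlay caches their distance, centroid offset, look-at quaternion and Object's transform.
; Each Tick, Object follows the midpoint, scales by the clamped distance ratio and rotates by the quaternion delta from the initial pose.
; An added twist around the hand-to-hand axis comes from both hands' right vectors against Object's up vector.
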(event `self.ReceiveBeginPlay`
  (set `self.InitialGrabDistance` (`KismetMathLibrary.VSize` (- (`SceneComponent.K2_GetComponentLocation` (`self.Right`)) (`SceneComponent.K2_GetComponentLocation` (`self.Left`)))))
  (bind _output_get (set `self.InitialCentroid` (* (+ (`SceneComponent.K2_GetComponentLocation` (`self.Right`)) (`SceneComponent.K2_GetComponentLocation` (`self.Left`))) 0.5)))
  (set `self.InitialMeshOffset` (- (`SceneComponent.K2_GetComponentLocation` (`self.Object`)) _output_get))
  (set `self.InitialScale` (`SceneComponent.K2_GetComponentScale` (`self.Object`)))
  (set `self.InitialObjectRotationQuat` (`KismetMathLibrary.Conv_RotatorToQuaternion` (`SceneComponent.K2_GetComponentRotation` (`self.Object`))))
  (bind _returnvalue (`LookAtRotationLibrary.FindLookAtQuaternion` (`SceneComponent.K2_GetComponentLocation` (`self.Right`)) (`SceneComponent.K2_GetComponentLocation` (`self.Left`)) (`SceneComponent.GetUpVector` (`self.Object`))))
  (bind _output_get_2 (set `self.InitialHandsRotationQuat` _returnvalue))
  (`SceneComponent.K2_SetWorldRotation` (`self.Object`) (`KismetMathLibrary.Quat_Rotator` _output_get_2) false false))

(event `self.ReceiveTick`
  (params (DeltaSeconds :type "Float (single-precision)"))
  (bind _initialscale_x (`KismetMathLibrary.BreakVector` (`self.InitialScale`)))
  (bind _returnvalue (`SceneComponent.GetUpVector` (`self.Object`)))
  (`SceneComponent.K2_SetWorldLocation` (`self.Object`) (+ (* (+ (`SceneComponent.K2_GetComponentLocation` (`self.Right`)) (`SceneComponent.K2_GetComponentLocation` (`self.Left`))) 0.5) (`self.InitialMeshOffset`)) false false)
  (bind _output_get (set `self.CurrentDistance` (`KismetMathLibrary.VSize` (- (`SceneComponent.K2_GetComponentLocation` (`self.Right`)) (`SceneComponent.K2_GetComponentLocation` (`self.Left`))))))
  (bind _output_get_2 (set `self.ScaleFactor` (/ _output_get (`self.InitialGrabDistance`))))
  (`SceneComponent.SetWorldScale3D` (`self.Object`) (`KismetMathLibrary.ClampVectorSize` (* _output_get_2 (`self.InitialScale`)) (/ _initialscale_x 5.0) (* _initialscale_x 5.0)))
  (bind _returnvalue_2 (`LookAtRotationLibrary.FindLookAtQuaternion` (`SceneComponent.K2_GetComponentLocation` (`self.Right`)) (`SceneComponent.K2_GetComponentLocation` (`self.Left`)) (`SceneComponent.GetUpVector` (`self.Object`))))
  (bind _output_get_3 (set `self.CırrentHandsRotationQuat` _returnvalue_2))
  (`SceneComponent.K2_SetWorldRotation` (`self.Object`) (`KismetMathLibrary.Quat_Rotator` (* (* _output_get_3 (`KismetMathLibrary.Quat_Inversed` (`self.InitialHandsRotationQuat`))) (`self.InitialObjectRotationQuat`))) false false)
  (`SceneComponent.K2_AddWorldRotation` (`self.Object`) (`KismetMathLibrary.RotatorFromAxisAndAngle` (`KismetMathLibrary.GetForwardVector` (`KismetMathLibrary.Quat_Rotator` (`self.CırrentHandsRotationQuat`))) (- (`KismetMathLibrary.DegAcos` (/ (+ (`KismetMathLibrary.Dot_VectorVector` _returnvalue (`SceneComponent.GetRightVector` (`self.Right`))) (`KismetMathLibrary.Dot_VectorVector` _returnvalue (`SceneComponent.GetRightVector` (`self.Left`)))) 2.0)) 90.0)) false false))

(fn `UserConstructionScript`)
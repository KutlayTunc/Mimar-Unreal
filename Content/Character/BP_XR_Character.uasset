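; XR player character for Meta Quest hand tracking with passthrough, driven by finger-pinch gestures.
; On BeginPlay with an HMD enabled, it sets resolution, tracking origin, passthrough and input mapping, then hands both hands to BPCGrabHelper.
; Index pinches start and stop grabs; middle pinches toggle a palm-socketed BP_PointerVisualizer per hand, switching that hand's grab type.
; Spectator camera spawning is disconnected, pending Meta's RGB camera access.
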(event Input|EnhancedActionEvents|EnhancedInputActionIA_R_MiddlePinch
  (params (ActionValue :type Boolean) (ElapsedSeconds :type Float%20%28double-precision%29) (TriggeredSeconds :type Float%20%28double-precision%29) (InputAction :type Input%20Action%20Object%20Reference :default "/Game/Inputs/FingersPinches/IA_R_MiddlePinch.IA_R_MiddlePinch"))
  (CallFunction|TogglePointer "HandRight"))

(event Input|EnhancedActionEvents|EnhancedInputActionIA_L_MiddlePinch
  (params (ActionValue :type Boolean) (ElapsedSeconds :type Float%20%28double-precision%29) (TriggeredSeconds :type Float%20%28double-precision%29) (InputAction :type Input%20Action%20Object%20Reference :default "/Game/Inputs/FingersPinches/IA_L_MiddlePinch.IA_L_MiddlePinch"))
  (CallFunction|TogglePointer "HandLeft"))

(event Input|EnhancedActionEvents|EnhancedInputActionIA_R_IndexPinch
  (params (ActionValue :type Boolean) (ElapsedSeconds :type Float%20%28double-precision%29) (TriggeredSeconds :type Float%20%28double-precision%29) (InputAction :type Input%20Action%20Object%20Reference :default "/Game/Inputs/FingersPinches/IA_R_IndexPinch.IA_R_IndexPinch"))
  (bind _bpc_grabhelper (Variables|Default|GetBPC_GrabHelper))
  (:Started
    (Default|RStartPinchGrab _bpc_grabhelper))
  (:Canceled
    (Default|RStopPinchGrab _bpc_grabhelper :!label _label))
  (:Completed
    (goto _label)))

(event Input|EnhancedActionEvents|EnhancedInputActionIA_L_IndexPinch
  (params (ActionValue :type Boolean) (ElapsedSeconds :type Float%20%28double-precision%29) (TriggeredSeconds :type Float%20%28double-precision%29) (InputAction :type Input%20Action%20Object%20Reference :default "/Game/Inputs/FingersPinches/IA_L_IndexPinch.IA_L_IndexPinch"))
  (bind _bpc_grabhelper (Variables|Default|GetBPC_GrabHelper))
  (:Started
    (Default|LStartPinchGrab _bpc_grabhelper))
  (:Canceled
    (Default|LStopPinchGrab _bpc_grabhelper :!label _label))
  (:Completed
    (goto _label)))

(event EventBeginPlay
  (CallFunction|AtBeginPlay))

(fn ConstructionScript)

(fn SetResolutionVR
  (Development|ExecuteConsoleCommand "xr.SecondaryScreenPercentage.HMDRenderTarget 100" 0)
  (Development|ExecuteConsoleCommand "vr.PixelDensity 1.0" 0))

(fn SpawnXRSpectator
  (bind _returnvalue (Game|SpawnActorfromClass "/Game/Core/XRSpectator/BP_XRSpectator.BP_XRSpectator_C" (Math|Transform|MakeTransform "0, 0, 0" "0, 0, 0" "1.000000,1.000000,1.000000") "Undefined" "MultiplyWithRoot" 0 0))
  (Default|StartCameraFollow _returnvalue (Variables|Default|GetCamera)))

(fn InitPassthrough
  (Class|OculusXRPassthroughSubsystem|InitializePersistentPassthrough (Subsystems|GetOculusXRPassthroughSubsystem)))

(fn SetHMDTrackingOrigin
  (Class|HeadMountedDisplayFunctionLibrary|SetTrackingOrigin "LocalFloor")
  (Development|PrintString (Utilities|String|Append "Tracking origin: " (Utilities|String|EnumtoString (Class|HeadMountedDisplayFunctionLibrary|GetTrackingOrigin)))))

(fn AtBeginPlay
  (if (Class|HeadMountedDisplayFunctionLibrary|IsHeadMountedDisplayEnabled)
    (Utilities|FlowControl|Sequence
      (:then_0
        (AtBeginPlay|SetResolutionVR))
      (:then_1
        (AtBeginPlay|SetHMDTrackingOrigin))
      (:then_2
        (AtBeginPlay|InitPassthrough))
      (:then_3
        (CallFunction|AddInputMappingContext))
      (:then_4
        (Default|SetReferences (Variables|Default|GetBPC_GrabHelper) self (Variables|Default|GetR_OculusXRHand) (Variables|Default|GetL_OculusXRHand))))))

(fn AddInputMappingContext
  (Input|AddMappingContext (PlayerController|LocalPlayerSubsystems|GetEnhancedInputLocalPlayerSubsystem (Game|GetPlayerController 0)) "/Game/Inputs/IMC_FingersPinches.IMC_FingersPinches" 0 "(bIgnoreAllPressedKeysUntilRelease=True,bForceImmediately=False,bNotifyUserSettings=False)"))

(fn TogglePointer
  (params (Hand :type EOculusXRHandType%20Enum :default "None"))
  (Utilities|IsValid (Utilities|Select :Index Hand :None 0 :HandLeft (Variables|Default|GetL_PointerRef) :HandRight (Variables|Default|GetR_PointerRef))
    (:Is%20Valid
      (LocalVariables|SetOldSpawnedActor (Utilities|Select :Index Hand :None 0 :HandLeft (Variables|Default|GetL_PointerRef) :HandRight (Variables|Default|GetR_PointerRef)))
      (Default|SetGrabType (Variables|Default|GetBPC_GrabHelper) Hand "NewEnumerator0")
      (Default|SetPointerVisualizer (Variables|Default|GetBPC_GrabHelper) Hand)
      (switch Utilities|FlowControl|Switch|SwitchonEOculusXRHandType Hand
        (:HandLeft
          (EventDispatchers|UnbindEventfromPointerLocationUpdated (LocalVariables|GetOldSpawnedActor) (EventDispatchers|CreateEvent (Variables|Default|GetBPC_GrabHelper) :!event LStartPointerGrab)))
        (:HandRight
          (EventDispatchers|UnbindEventfromPointerLocationUpdated (LocalVariables|GetOldSpawnedActor) (EventDispatchers|CreateEvent (Variables|Default|GetBPC_GrabHelper) :!event RStartPointerGrab))))
      (Actor|DestroyActor (LocalVariables|GetOldSpawnedActor))
      (Default|SetGrabType (Variables|Default|GetBPC_GrabHelper) Hand "NewEnumerator0"))
    (:Is%20Not%20Valid
      (bind _returnvalue (Game|SpawnActorfromClass "/Game/VFX/Blueprints/BP_PointerVisualizer.BP_PointerVisualizer_C" (Math|Transform|MakeTransform "0, 0, 0" "0, 0, 0" "1.000000,1.000000,1.000000") "Undefined" "OverrideRootScale" self Hand 0))
      (bind _output_get (LocalVariables|SetNewSpawnedActor _returnvalue))
      (Default|SetPointerVisualizer (Variables|Default|GetBPC_GrabHelper) Hand _output_get)
      (Default|SetGrabType (Variables|Default|GetBPC_GrabHelper) Hand "NewEnumerator1")
      (switch Utilities|FlowControl|Switch|SwitchonEOculusXRHandType Hand
        (:HandLeft
          (bind _output_get_2 (Variables|Default|SetL_PointerRef (LocalVariables|GetNewSpawnedActor)))
          (Transformation|AttachComponentToComponent _output_get_2 (Variables|Default|GetL_OculusXRHand) "palmPointerSocket" "SnapToTarget" "SnapToTarget" "KeepWorld" false)
          (EventDispatchers|BindEventtoPointerLocationUpdated (LocalVariables|GetNewSpawnedActor) (EventDispatchers|CreateEvent (Variables|Default|GetBPC_GrabHelper) :!event LStartPointerGrab)))
        (:HandRight
          (bind _output_get_3 (Variables|Default|SetR_PointerRef (LocalVariables|GetNewSpawnedActor)))
          (Transformation|AttachComponentToComponent _output_get_3 (Variables|Default|GetR_OculusXRHand) "palmPointerSocket" "SnapToTarget" "SnapToTarget" "KeepWorld" false)
          (EventDispatchers|BindEventtoPointerLocationUpdated (LocalVariables|GetNewSpawnedActor) (EventDispatchers|CreateEvent (Variables|Default|GetBPC_GrabHelper) :!event RStartPointerGrab)))))))

(fn PassRefstoGrabHelper)